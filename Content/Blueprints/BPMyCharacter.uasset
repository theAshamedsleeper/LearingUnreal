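; BPMyCharacter is a character Blueprint that picks a random Manny or Quinn mesh and collapses into a ragdoll on death.
; The Construction Script sets the mesh and zeroes Health for an instant ragdoll, and the Hit event also zeroes Health.
; Tick polls Die, which clears IsAlive and enables mesh physics once Health is depleted.
; An unused FindRange event prints the distance to the first Enemy-tagged actor.
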(event Custom|Die
  ;[1 1 1] Set Ragdoll, checks health
  (if (and (Variables|Default|GetIsAlive) (<= (Variables|Default|Gethealth) 0))
    (Variables|Default|SetIsAlive false)
    (Physics|SetSimulatePhysics (Variables|Character|GetMesh) true)))

(event Custom|FindRange
  ;[1 1 1] Get Range
  (bind _outactors (Actor|GetAllActorswithTag "Enemy"))
  (Development|PrintString (Utilities|String|ToString(Float) (Transformation|GetDistanceTo (Utilities|Array|Get(acopy) _outactors) self))))

(event Collision|EventActorBeginOverlap
  (params (OtherActor :type Actor%20Object%20Reference)))

(event EventTick
  (params (DeltaSeconds :type Float%20%28single-precision%29))
  (CallFunction|Die))

(event Collision|EventHit
  (params (MyComp :type Primitive%20Component%20Object%20Reference) (Other :type Actor%20Object%20Reference) (OtherComp :type Primitive%20Component%20Object%20Reference) (bSelfMoved :type Boolean) (HitLocation :type Vector :default "0, 0, 0") (HitNormal :type Vector :default "0, 0, 0") (NormalImpulse :type Vector :default "0, 0, 0") (Hit :type Hit%20Result%20Structure%20%28by%20ref%29))
  (Variables|Default|Sethealth 0))

(event EventBeginPlay)

(fn ConstructionScript
  (bind _array (Utilities|Array|MakeArray "/Game/ControlRig/Characters/Mannequins/Meshes/SKM_Manny.SKM_Manny" "/Game/ControlRig/Characters/Mannequins/Meshes/SKM_Manny_Simple.SKM_Manny_Simple" "/Game/ControlRig/Characters/Mannequins/Meshes/SKM_Quinn.SKM_Quinn" "/Game/ControlRig/Characters/Mannequins/Meshes/SKM_Quinn_Simple.SKM_Quinn_Simple"))
  ;[1 1 1] Random Skeletal mesh
  (Components|SkeletalMesh|SetSkeletalMeshAsset (Variables|Character|GetMesh) (Utilities|Array|Get(acopy) _array (Math|Random|RandomInteger (Utilities|Array|Length _array))))
  (Variables|Default|Sethealth 0) ; Set to 0 for instant Ragdoll
)